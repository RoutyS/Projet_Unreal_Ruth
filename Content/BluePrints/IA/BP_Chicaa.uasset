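; BP_Chicaa is an AI character that attacks the player by throwing muffins.
; Its PlayerChase event calls Feu, which stops movement immediately, turns the character on yaw toward player 0, and spawns a BP_Muffin at the MuffinSpawner transform.
; BeginPlay, overlap and Tick are disabled stubs, and nothing in this graph triggers PlayerChase.
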(event Custom|Feu
  (Components|Movement|StopMovementImmediately (Variables|Character|GetCharacterMovement))
  (Transformation|SetActorRotation (Math|Rotator|MakeRotator 0.0 0.0 (.yaw (Math|Rotator|FindLookatRotation (Transformation|GetActorLocation) (Transformation|GetActorLocation (Game|GetPlayerCharacter 0))))))
  (Game|SpawnActorfromClass "/Game/BluePrints/FirstPerson/Blueprints/Munitions/BP_Muffin.BP_Muffin_C" (Transformation|GetWorldTransform (Variables|Default|GetMuffinSpawner)) "Undefined" "MultiplyWithRoot" 0 1e+01 0))

(event EventBeginPlay
  (|CallParentFunction) ; This node is disabled and will not be called.\nDrag off pins to build functionality.
)

(event Collision|EventActorBeginOverlap
  (params (OtherActor :type Actor%20Object%20Reference))
  (|CallParentFunction OtherActor) ; This node is disabled and will not be called.\nDrag off pins to build functionality.
)

(event EventTick
  (params (DeltaSeconds :type Float%20%28single-precision%29))
  (|CallParentFunction DeltaSeconds) ; This node is disabled and will not be called.\nDrag off pins to build functionality.
)

(event EventPlayerChase
  (params (Player :type Pawn%20Object%20Reference))
  (CallFunction|Feu))

(fn ConstructionScript
  (|CallParentFunction))