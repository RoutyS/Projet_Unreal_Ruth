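; AI chaser character that pursues the player, deals damage on contact, then runs off.
; PlayerChase moves it to the given actor and resumes patrol on success, while a Box overlap with BP_FirstPersonCharacter calls TakeDamage and RunAway.
; RunAway boosts walk speed and uses twice the self-to-player vector as an absolute destination.
; Either move result returns to patrol and calls the empty audio event; the speed reset is disabled.
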(event OnComponentBeginOverlap(Box)
  (params (OverlappedComponent :type Primitive%20Component%20Object%20Reference) (OtherActor :type Actor%20Object%20Reference) (OtherComp :type Primitive%20Component%20Object%20Reference) (OtherBodyIndex :type Integer) (bFromSweep :type Boolean) (SweepResult :type Hit%20Result%20Structure%20%28by%20ref%29))
  (bind _asbp_first_person_character (Utilities|Casting|CastToBP_FirstPersonCharacter OtherActor))
  (Default|TakeDamage _asbp_first_person_character)
  (CallFunction|RunAway))

(event Custom|RunAway
  (Variables|/Script/Engine.CharacterMovementComponent|SetMaxWalkSpeed (Variables|Character|GetCharacterMovement) 3e+03)
  (AI|AIMoveTo self (* (- (Transformation|GetActorLocation (Game|GetPlayerCharacter 0)) (Transformation|GetActorLocation)) 2) 0 5.0 false
    (:OnSuccess
      _)
    (:OnFail
      _))
  (Variables|/Script/Engine.CharacterMovementComponent|SetMaxWalkSpeed (Variables|Character|GetCharacterMovement) 1.7e+02)
  (CallFunction|ReturntoPatrol)
  (CallFunction|JouerAudio))

(event Custom|jouerAudio)

(event EventBeginPlay
  (|CallParentFunction) ; This node is disabled and will not be called.\nDrag off pins to build functionality.
)

(event Collision|EventActorBeginOverlap
  (params (OtherActor :type Actor%20Object%20Reference)))

(event EventTick
  (params (DeltaSeconds :type Float%20%28single-precision%29))
  (|CallParentFunction DeltaSeconds) ; This node is disabled and will not be called.\nDrag off pins to build functionality.
)

(event EventPlayerChase
  (params (Player :type Pawn%20Object%20Reference))
  (AI|AIMoveTo self "0, 0, 0" Player 1.0 false
    (:OnSuccess
      (CallFunction|ReturntoPatrol))))

(fn ConstructionScript
  (|CallParentFunction))