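; Master AI character that patrols, seeks the player's last known location and provides a bullet-firing attack.
; Patrol loops through random reachable points with pauses; seeking doubles its search radius until an iteration limit returns it to patrol.
; Fire stops movement, faces the player, spawns BP_Bullet, then rechecks sight and range after reloading.
; Pawn sensing calls PlayerChase, which is empty here, and the logic setting CanSeePlayer is disconnected.
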(event OnSeePawn(PawnSensing)
  (params (Pawn :type Pawn%20Object%20Reference))
  ;[1 1 1] If we see player and we are not in range get closer to fire - if we don't see player seek for him or patrol
  (if (== Pawn (Game|GetPlayerCharacter 0))
    (CallFunction|PlayerChase (Game|GetPlayerCharacter 0))))

(event Custom|ReturnToPatrol
  (bind _returnvalue (Transformation|GetActorLocation))
  (bind _radiuspatrol (Variables|RadiusRandom|GetRadiusPatrol))
  (bind _randomlocation (AI|Navigation|GetRandomReachablePointinRadius _returnvalue _radiuspatrol 0 0))
  ;[1 1 1] Patrol - Get random point in area
  (Development|PrintString "Return to patrol")
  (Variables|NbSeekIteraction|Setnb_seekPlayer 0)
  (Rendering|Debug|DrawDebugCircle _randomlocation 0.0 12 "(R=0.213068,G=0.193599,B=1.000000,A=1.000000)" 1e+01 0.0 "0.000000,1.000000,0.000000" "0.000000,0.000000,1.000000" true)
  (AI|AIMoveTo self _randomlocation 0 5.0 true
    (:OnSuccess
      _)
    (:OnFail
      _))
  (Utilities|FlowControl|Delay (Math|Random|RandomFloatinRange 2.0 5.0))
  (CallFunction|ReturntoPatrol))

(event Custom|PlayerChase
  (params (Player :type Pawn%20Object%20Reference)))

(event Custom|SeePlayerMoveTo
  (params (Last%20seen%20Player%20Location :type Vector))
  (bind _radiuslookingforplayer (Variables|RadiusRandom|GetRadiusLookingForPlayer))
  (bind _randomlocation (AI|Navigation|GetRandomReachablePointinRadius Last%20seen%20Player%20Location _radiuslookingforplayer 0 0))
  ;[1 1 1] Get a random point in a radius from last seen player location - move ia to the random point
  (Development|PrintString "seekPlayerMoveTo")
  (AI|AIMoveTo self _randomlocation 0 5.0 false
    (:OnSuccess
      _)
    (:OnFail
      _))
  (CallFunction|CheckCanSeePlayerFireGunRange _randomlocation))

(event Custom|GoToPayerLocation_NotGunRange
  (params (Last%20Player%20Location :type Vector))
  ;[1 1 1] move ia to last seen player location
  (AI|AIMoveTo self Last%20Player%20Location 0 (Variables|FireRangeDefault|GetgunRange) false
    (:then
      (Variables|Perception|Setmoving? true))
    (:OnSuccess
      (Variables|Perception|Setmoving? false :!label _label)
      (CallFunction|CheckCanSeePlayerFireGunRange Last%20Player%20Location))
    (:OnFail
      (goto _label))))

(event Custom|SeekPlayer
  (params (Last%20Seen%20Player%20Location :type Vector))
  ;[1 1 1] increase radius random point
  (Utilities|FlowControl|Delay (Math|Random|RandomFloatinRange 2.0 5.0))
  (Development|PrintString "seekplayer")
  (Variables|RadiusRandom|SetRadiusLookingForPlayer (* (Variables|RadiusRandom|GetRadiusLookingForPlayer) 2.0))
  (bind _result (Math|Integer|IncrementInt (Variables|NbSeekIteraction|Getnb_seekPlayer))
    (:%20%20
      (if (>= _result (Variables|NbSeekIteraction|Getnb_seekPlayerIterationMax))
        (CallFunction|ReturntoPatrol)
        (else
          (CallFunction|SeePlayerMoveto Last%20Seen%20Player%20Location))))))

(event Custom|Fire
  ;[1 1 1] Fire Bulett - stop movment - rotate to player - spawn bp bullet
  (Components|Movement|StopMovementImmediately (Variables|Character|GetCharacterMovement))
  (Transformation|SetActorRotation (Math|Rotator|MakeRotator 0.0 0.0 (.yaw (Math|Rotator|FindLookatRotation (Transformation|GetActorLocation) (Transformation|GetActorLocation (Game|GetPlayerCharacter 0))))))
  (Game|SpawnActorfromClass "/Game/BluePrints/FirstPerson/Blueprints/Munitions/BP_Bullet.BP_Bullet_C" (Transformation|GetWorldTransform (Variables|Default|GetTarget)) "Undefined" "MultiplyWithRoot" 0 (Variables|GunFire|GetbulletDammage) 0)
  (Utilities|FlowControl|Delay (Variables|GunFire|GetreloadDelay))
  (CallFunction|CheckCanSeePlayerFireGunRange (Transformation|GetActorLocation)))

(event EventBeginPlay
  ;[1 1 1] Comment
  (CallFunction|ReturntoPatrol)
  (switch Utilities|FlowControl|Switch|SwitchonE_IA_Type (Variables|CharacterInfo|GetIA_Type)))

(event EventTick
  (params (DeltaSeconds :type Float%20%28single-precision%29)))

(fn ConstructionScript)

(fn CheckCanSeePlayerFireGunRange
  (params (Last%20Seen%20Player%20Location :type Vector))
  (if (Variables|Perception|GetcanSeePlayer?)
    (Utilities|AmIinGunRange?
      (:im%20no%20in%20range
        _)))
  (CallFunction|SeekPlayer Last%20Seen%20Player%20Location))

(fn RotatetoPlayer
  (if (Variables|Perception|GetcanSeePlayer?)
    (Transformation|SetActorRotation (Math|Rotator|FindLookatRotation (Transformation|GetActorLocation) (Transformation|GetActorLocation (Game|GetPlayerCharacter 0))))
    (else
      (Utilities|Time|ClearTimerbyFunctionName 0 "RotateToPlayer"))))