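; BP_MasterBonus is a pickup that grants one of two ammo types or health to BP_FirstPersonCharacter, chosen by its bonus type.
; Sphere overlap applies the bonus, plays brief smoke and sound calls, then hides the actor and disables collision.
; After a cooldown it reappears with collision restored and spawns another short-lived emitter, which has no template set.
; The Tick movement logic is unfinished and never runs.
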(event OnComponentBeginOverlap(Sphere)
  (params (OverlappedComponent :type Primitive%20Component%20Object%20Reference) (OtherActor :type Actor%20Object%20Reference) (OtherComp :type Primitive%20Component%20Object%20Reference) (OtherBodyIndex :type Integer) (bFromSweep :type Boolean) (SweepResult :type Hit%20Result%20Structure%20%28by%20ref%29))
  (bind _asbp_first_person_character (Utilities|Casting|CastToBP_FirstPersonCharacter OtherActor))
  (switch Utilities|FlowControl|Switch|SwitchonE_BonusType (Variables|Default|GetE_BonusType)
    (:NewEnumerator0
      (Default|AddBulletsR _asbp_first_person_character (Variables|Default|GetBullets%20to%20Add_R)))
    (:NewEnumerator1
      (Default|AddHealth _asbp_first_person_character (Variables|Default|GetHealth%20to%20Add)))
    (:NewEnumerator3
      (Default|AddBulletsB _asbp_first_person_character (Variables|Default|GetBullets%20to%20Add_B))))
  (bind _returnvalue (Effects|SpawnEmitteratLocation "/Game/StarterContent/Particles/P_Smoke.P_Smoke" (Transformation|GetActorLocation) "0, 0, 0" "5.000000,5.000000,5.000000"))
  (Utilities|FlowControl|Sequence
    (:then_0
      (Utilities|FlowControl|Delay 0.2)
      (Components|DestroyComponent _returnvalue))
    (:then_1
      (Audio|PlaySoundatLocation 0 (Transformation|GetActorLocation) "0, 0, 0" 1.0 1.0 0.0 0 0 0 0))
    (:then_2
      (Rendering|SetActorHiddenInGame true)
      (Collision|SetActorEnableCollision false))
    (:then_3
      (Utilities|FlowControl|Delay (Variables|Default|GetCoolDownBonus))
      (Rendering|SetActorHiddenInGame false)
      (Collision|SetActorEnableCollision true)
      (bind _returnvalue_2 (Effects|SpawnEmitteratLocation 0 (Transformation|GetActorLocation) "0, 0, 0" "5.000000,5.000000,5.000000"))
      (Utilities|FlowControl|Delay 0.2)
      (Components|DestroyComponent _returnvalue_2))))

(event EventTick
  (params (DeltaSeconds :type Float%20%28single-precision%29))
  ;[1 1 1] mouvement
)

(fn ConstructionScript)